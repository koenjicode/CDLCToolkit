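; Actor that assembles a modular character from a CreationPart's skeletal meshes and colours it, entirely in the construction script.
; Default meshes, resolved by asset-registry path, fill body, optional and racial slot components, then the selected MeshVariation's meshes override them.
; Each child mesh material becomes a dynamic instance receiving four colour/pattern slots via ColorDataFunc.
; That function skips non-skin eyebrow and beard materials and redirects skin materials onto MFace.
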(event EventBeginPlay)

(event Collision|EventActorBeginOverlap
  (params (OtherActor :type Actor%20Object%20Reference)))

(event EventTick
  (params (DeltaSeconds :type Float%20%28single-precision%29)))

(fn ConstructionScript
  (bind _creationpart (Variables|MeshData|GetCreationPart))
  (bind _mesh_variation (Variables|MeshData|GetMesh%20Variation))
  (for _array_element (Variables|/Script/LuxorGame.LuxCreationImportedPart|GetDefaultMeshes (Utilities|ResolveSoftReference _creationpart))
    (bind _asskeletal_mesh (Utilities|Casting|CastToSkeletalMesh (Class|AssetRegistryHelpers|GetAsset (Class|AssetRegistry|GetAssetbyObjectPath (Class|AssetRegistryHelpers|GetAssetRegistry) (Utilities|String|StringToName (Utilities|Struct|BreakStringAssetReference (.MeshRef (Utilities|Struct|BreakLuxSlotMeshData _array_element)))) false))))
    (if (Utilities|Enum|Equal(Enum) (.Slot (Utilities|Struct|BreakLuxSlotMeshData _array_element)) "EPS_Mandatory_Face")
      (Class|SkinnedMeshComponent|SetSkeletalMesh (Variables|Default|GetM_Face) _asskeletal_mesh true)
      (elif (Utilities|Enum|Equal(Enum) (.Slot (Utilities|Struct|BreakLuxSlotMeshData _array_element)) "EPS_Mandatory_Scalp")
        (Class|SkinnedMeshComponent|SetSkeletalMesh (Variables|Default|GetM_Scalp) _asskeletal_mesh true)
        (elif (Utilities|Enum|Equal(Enum) (.Slot (Utilities|Struct|BreakLuxSlotMeshData _array_element)) "EPS_Mandatory_Neck")
          (Class|SkinnedMeshComponent|SetSkeletalMesh (Variables|Default|GetM_Neck) _asskeletal_mesh true)
          (elif (Utilities|Enum|Equal(Enum) (.Slot (Utilities|Struct|BreakLuxSlotMeshData _array_element)) "EPS_Mandatory_Hair")
            (Class|SkinnedMeshComponent|SetSkeletalMesh (Variables|Default|GetM_Hair) _asskeletal_mesh true)
            (elif (Utilities|Enum|Equal(Enum) (.Slot (Utilities|Struct|BreakLuxSlotMeshData _array_element)) "EPS_Mandatory_Hip")
              (Class|SkinnedMeshComponent|SetSkeletalMesh (Variables|Default|GetM_Hip) _asskeletal_mesh true)
              (elif (Utilities|Enum|Equal(Enum) (.Slot (Utilities|Struct|BreakLuxSlotMeshData _array_element)) "EPS_Mandatory_Stomach")
                (Class|SkinnedMeshComponent|SetSkeletalMesh (Variables|Default|GetM_Stomach) _asskeletal_mesh true)
                (elif (Utilities|Enum|Equal(Enum) (.Slot (Utilities|Struct|BreakLuxSlotMeshData _array_element)) "EPS_Mandatory_Chest")
                  (Class|SkinnedMeshComponent|SetSkeletalMesh (Variables|Default|GetM_Chest) _asskeletal_mesh true)
                  (elif (Utilities|Enum|Equal(Enum) (.Slot (Utilities|Struct|BreakLuxSlotMeshData _array_element)) "EPS_Mandatory_Tanima")
                    (Class|SkinnedMeshComponent|SetSkeletalMesh (Variables|Default|GetM_Tanima) _asskeletal_mesh true)
                    (elif (Utilities|Enum|Equal(Enum) (.Slot (Utilities|Struct|BreakLuxSlotMeshData _array_element)) "EPS_Mandatory_Hand")
                      (Class|SkinnedMeshComponent|SetSkeletalMesh (Variables|Default|GetM_Hand) _asskeletal_mesh true)
                      (elif (Utilities|Enum|Equal(Enum) (.Slot (Utilities|Struct|BreakLuxSlotMeshData _array_element)) "EPS_Mandatory_Elbow")
                        (Class|SkinnedMeshComponent|SetSkeletalMesh (Variables|Default|GetM_Elbow) _asskeletal_mesh true)
                        (elif (Utilities|Enum|Equal(Enum) (.Slot (Utilities|Struct|BreakLuxSlotMeshData _array_element)) "EPS_Mandatory_ForeArm")
                          (Class|SkinnedMeshComponent|SetSkeletalMesh (Variables|Default|GetM_ForeArm) _asskeletal_mesh true)
                          (elif (Utilities|Enum|Equal(Enum) (.Slot (Utilities|Struct|BreakLuxSlotMeshData _array_element)) "EPS_Mandatory_UpperArm")
                            (Class|SkinnedMeshComponent|SetSkeletalMesh (Variables|Default|GetM_UpperArm) _asskeletal_mesh true)
                            (elif (Utilities|Enum|Equal(Enum) (.Slot (Utilities|Struct|BreakLuxSlotMeshData _array_element)) "EPS_Mandatory_Shin")
                              (Class|SkinnedMeshComponent|SetSkeletalMesh (Variables|Default|GetM_Shin) _asskeletal_mesh true)
                              (elif (Utilities|Enum|Equal(Enum) (.Slot (Utilities|Struct|BreakLuxSlotMeshData _array_element)) "EPS_Mandatory_Thigh")
                                (Class|SkinnedMeshComponent|SetSkeletalMesh (Variables|Default|GetM_Thigh) _asskeletal_mesh true)
                                (elif (Utilities|Enum|Equal(Enum) (.Slot (Utilities|Struct|BreakLuxSlotMeshData _array_element)) "EPS_Mandatory_Knee")
                                  (Class|SkinnedMeshComponent|SetSkeletalMesh (Variables|Default|GetM_Knee) _asskeletal_mesh true)
                                  (elif (Utilities|Enum|Equal(Enum) (.Slot (Utilities|Struct|BreakLuxSlotMeshData _array_element)) "EPS_Mandatory_Ankle")
                                    (Class|SkinnedMeshComponent|SetSkeletalMesh (Variables|Default|GetM_Ankle) _asskeletal_mesh true)
                                    (elif (Utilities|Enum|Equal(Enum) (.Slot (Utilities|Struct|BreakLuxSlotMeshData _array_element)) "EPS_Optional_Head")
                                      (Class|SkinnedMeshComponent|SetSkeletalMesh (Variables|Default|GetO_Head) _asskeletal_mesh true)
                                      (elif (Utilities|Enum|Equal(Enum) (.Slot (Utilities|Struct|BreakLuxSlotMeshData _array_element)) "EPS_Optional_Glasses")
                                        (Class|SkinnedMeshComponent|SetSkeletalMesh (Variables|Default|GetO_Glasses) _asskeletal_mesh true)
                                        (elif (Utilities|Enum|Equal(Enum) (.Slot (Utilities|Struct|BreakLuxSlotMeshData _array_element)) "EPS_Optional_Necklace")
                                          (Class|SkinnedMeshComponent|SetSkeletalMesh (Variables|Default|GetO_Necklace) _asskeletal_mesh true)
                                          (elif (Utilities|Enum|Equal(Enum) (.Slot (Utilities|Struct|BreakLuxSlotMeshData _array_element)) "EPS_Optional_ChestFit")
                                            (Class|SkinnedMeshComponent|SetSkeletalMesh (Variables|Default|GetO_ChestFit) _asskeletal_mesh true)
                                            (elif (Utilities|Enum|Equal(Enum) (.Slot (Utilities|Struct|BreakLuxSlotMeshData _array_element)) "EPS_Optional_ChestPlate")
                                              (Class|SkinnedMeshComponent|SetSkeletalMesh (Variables|Default|GetO_ChestPlate) _asskeletal_mesh true)
                                              (elif (Utilities|Enum|Equal(Enum) (.Slot (Utilities|Struct|BreakLuxSlotMeshData _array_element)) "EPS_Optional_BackCloth")
                                                (Class|SkinnedMeshComponent|SetSkeletalMesh (Variables|Default|GetO_BackCloth) _asskeletal_mesh true)
                                                (elif (Utilities|Enum|Equal(Enum) (.Slot (Utilities|Struct|BreakLuxSlotMeshData _array_element)) "EPS_Optional_UpperArm")
                                                  (Class|SkinnedMeshComponent|SetSkeletalMesh (Variables|Default|GetO_UpperArm) _asskeletal_mesh true)
                                                  (elif (Utilities|Enum|Equal(Enum) (.Slot (Utilities|Struct|BreakLuxSlotMeshData _array_element)) "EPS_Optional_Shoulder")
                                                    (Class|SkinnedMeshComponent|SetSkeletalMesh (Variables|Default|GetO_Shoulder) _asskeletal_mesh true)
                                                    (elif (Utilities|Enum|Equal(Enum) (.Slot (Utilities|Struct|BreakLuxSlotMeshData _array_element)) "EPS_Optional_Gauntlet")
                                                      (Class|SkinnedMeshComponent|SetSkeletalMesh (Variables|Default|GetO_Gauntlet) _asskeletal_mesh true)
                                                      (elif (Utilities|Enum|Equal(Enum) (.Slot (Utilities|Struct|BreakLuxSlotMeshData _array_element)) "EPS_Optional_UpperLeg")
                                                        (Class|SkinnedMeshComponent|SetSkeletalMesh (Variables|Default|GetO_UpperLeg) _asskeletal_mesh true)
                                                        (elif (Utilities|Enum|Equal(Enum) (.Slot (Utilities|Struct|BreakLuxSlotMeshData _array_element)) "EPS_Optional_Skirt")
                                                          (Class|SkinnedMeshComponent|SetSkeletalMesh (Variables|Default|GetO_Skirt) _asskeletal_mesh true)
                                                          (elif (Utilities|Enum|Equal(Enum) (.Slot (Utilities|Struct|BreakLuxSlotMeshData _array_element)) "EPS_Optional_Hem")
                                                            (Class|SkinnedMeshComponent|SetSkeletalMesh (Variables|Default|GetO_Hem) _asskeletal_mesh true)
                                                            (elif (Utilities|Enum|Equal(Enum) (.Slot (Utilities|Struct|BreakLuxSlotMeshData _array_element)) "EPS_Optional_Belt")
                                                              (Class|SkinnedMeshComponent|SetSkeletalMesh (Variables|Default|GetO_Belt) _asskeletal_mesh true)
                                                              (elif (Utilities|Enum|Equal(Enum) (.Slot (Utilities|Struct|BreakLuxSlotMeshData _array_element)) "EPS_Optional_Shoes")
                                                                (Class|SkinnedMeshComponent|SetSkeletalMesh (Variables|Default|GetO_Shoes) _asskeletal_mesh true)
                                                                (elif (Utilities|Enum|Equal(Enum) (.Slot (Utilities|Struct|BreakLuxSlotMeshData _array_element)) "EPS_Optional_UnderShin")
                                                                  (Class|SkinnedMeshComponent|SetSkeletalMesh (Variables|Default|GetO_UnderShin) _asskeletal_mesh true)
                                                                  (elif (Utilities|Enum|Equal(Enum) (.Slot (Utilities|Struct|BreakLuxSlotMeshData _array_element)) "EPS_Optional_Accessory")
                                                                    (Class|SkinnedMeshComponent|SetSkeletalMesh (Variables|Default|GetO_Accessory) _asskeletal_mesh true)
                                                                    (elif (Utilities|Enum|Equal(Enum) (.Slot (Utilities|Struct|BreakLuxSlotMeshData _array_element)) "EPS_Optional_Cheek")
                                                                      (Class|SkinnedMeshComponent|SetSkeletalMesh (Variables|Default|GetO_Cheek) _asskeletal_mesh true)
                                                                      (elif (Utilities|Enum|Equal(Enum) (.Slot (Utilities|Struct|BreakLuxSlotMeshData _array_element)) "EPS_Optional_Mantle")
                                                                        (Class|SkinnedMeshComponent|SetSkeletalMesh (Variables|Default|GetO_Mantle) _asskeletal_mesh true)
                                                                        (elif (Utilities|Enum|Equal(Enum) (.Slot (Utilities|Struct|BreakLuxSlotMeshData _array_element)) "EPS_Optional_Maegami1")
                                                                          (Class|SkinnedMeshComponent|SetSkeletalMesh (Variables|Default|GetO_OptionalBangs1) _asskeletal_mesh true)
                                                                          (elif (Utilities|Enum|Equal(Enum) (.Slot (Utilities|Struct|BreakLuxSlotMeshData _array_element)) "EPS_Optional_Maegami2")
                                                                            (Class|SkinnedMeshComponent|SetSkeletalMesh (Variables|Default|GetO_OptionalBangs2) _asskeletal_mesh true)
                                                                            (elif (Utilities|Enum|Equal(Enum) (.Slot (Utilities|Struct|BreakLuxSlotMeshData _array_element)) "EPS_Racial_1")
                                                                              (Class|SkinnedMeshComponent|SetSkeletalMesh (Variables|Default|GetRacial1) _asskeletal_mesh true)
                                                                              (elif (Utilities|Enum|Equal(Enum) (.Slot (Utilities|Struct|BreakLuxSlotMeshData _array_element)) "EPS_Racial_2")
                                                                                (Class|SkinnedMeshComponent|SetSkeletalMesh (Variables|Default|GetRacial2) _asskeletal_mesh true)
                                                                                (elif (Utilities|Enum|Equal(Enum) (.Slot (Utilities|Struct|BreakLuxSlotMeshData _array_element)) "EPS_Racial_3")
                                                                                  (Class|SkinnedMeshComponent|SetSkeletalMesh (Variables|Default|GetRacial3) _asskeletal_mesh true)
                                                                                  (elif (Utilities|Enum|Equal(Enum) (.Slot (Utilities|Struct|BreakLuxSlotMeshData _array_element)) "EPS_Racial_4")
                                                                                    (Class|SkinnedMeshComponent|SetSkeletalMesh (Variables|Default|GetRacial4) _asskeletal_mesh true))))))))))))))))))))))))))))))))))))))))))
  (for _array_element_2 (Variables|/Script/LuxorGame.LuxCreationImportedPart|GetMeshVariations (Utilities|ResolveSoftReference _creationpart))
    (if (Utilities|Enum|Equal(Enum) (.Variation (Utilities|Struct|BreakLuxMeshDataVariation _array_element_2)) "EPV_A")
      (if (Utilities|Enum|Equal(Enum) _mesh_variation "EPV_A")
        (for _array_element_3 (.SlotMeshData (Utilities|Struct|BreakLuxMeshDataVariation _array_element_2)) :!label _label
          (bind _asskeletal_mesh_2 (Utilities|Casting|CastToSkeletalMesh (Class|AssetRegistryHelpers|GetAsset (Class|AssetRegistry|GetAssetbyObjectPath (Class|AssetRegistryHelpers|GetAssetRegistry) (Utilities|String|StringToName (Utilities|Struct|BreakStringAssetReference (.MeshRef (Utilities|Struct|BreakLuxSlotMeshData _array_element_3)))) false))))
          (if (Utilities|Enum|Equal(Enum) (.Slot (Utilities|Struct|BreakLuxSlotMeshData _array_element_3)) "EPS_Mandatory_Face")
            (Class|SkinnedMeshComponent|SetSkeletalMesh (Variables|Default|GetM_Face) _asskeletal_mesh_2 true)
            (elif (Utilities|Enum|Equal(Enum) (.Slot (Utilities|Struct|BreakLuxSlotMeshData _array_element_3)) "EPS_Mandatory_Scalp")
              (Class|SkinnedMeshComponent|SetSkeletalMesh (Variables|Default|GetM_Scalp) _asskeletal_mesh_2 true)
              (elif (Utilities|Enum|Equal(Enum) (.Slot (Utilities|Struct|BreakLuxSlotMeshData _array_element_3)) "EPS_Mandatory_Neck")
                (Class|SkinnedMeshComponent|SetSkeletalMesh (Variables|Default|GetM_Neck) _asskeletal_mesh_2 true)
                (elif (Utilities|Enum|Equal(Enum) (.Slot (Utilities|Struct|BreakLuxSlotMeshData _array_element_3)) "EPS_Mandatory_Hair")
                  (Class|SkinnedMeshComponent|SetSkeletalMesh (Variables|Default|GetM_Hair) _asskeletal_mesh_2 true)
                  (elif (Utilities|Enum|Equal(Enum) (.Slot (Utilities|Struct|BreakLuxSlotMeshData _array_element_3)) "EPS_Mandatory_Hip")
                    (Class|SkinnedMeshComponent|SetSkeletalMesh (Variables|Default|GetM_Hip) _asskeletal_mesh_2 true)
                    (elif (Utilities|Enum|Equal(Enum) (.Slot (Utilities|Struct|BreakLuxSlotMeshData _array_element_3)) "EPS_Mandatory_Stomach")
                      (Class|SkinnedMeshComponent|SetSkeletalMesh (Variables|Default|GetM_Stomach) _asskeletal_mesh_2 true)
                      (elif (Utilities|Enum|Equal(Enum) (.Slot (Utilities|Struct|BreakLuxSlotMeshData _array_element_3)) "EPS_Mandatory_Chest")
                        (Class|SkinnedMeshComponent|SetSkeletalMesh (Variables|Default|GetM_Chest) _asskeletal_mesh_2 true)
                        (elif (Utilities|Enum|Equal(Enum) (.Slot (Utilities|Struct|BreakLuxSlotMeshData _array_element_3)) "EPS_Mandatory_Tanima")
                          (Class|SkinnedMeshComponent|SetSkeletalMesh (Variables|Default|GetM_Tanima) _asskeletal_mesh_2 true)
                          (elif (Utilities|Enum|Equal(Enum) (.Slot (Utilities|Struct|BreakLuxSlotMeshData _array_element_3)) "EPS_Mandatory_Hand")
                            (Class|SkinnedMeshComponent|SetSkeletalMesh (Variables|Default|GetM_Hand) _asskeletal_mesh_2 true)
                            (elif (Utilities|Enum|Equal(Enum) (.Slot (Utilities|Struct|BreakLuxSlotMeshData _array_element_3)) "EPS_Mandatory_Elbow")
                              (Class|SkinnedMeshComponent|SetSkeletalMesh (Variables|Default|GetM_Elbow) _asskeletal_mesh_2 true)
                              (elif (Utilities|Enum|Equal(Enum) (.Slot (Utilities|Struct|BreakLuxSlotMeshData _array_element_3)) "EPS_Mandatory_ForeArm")
                                (Class|SkinnedMeshComponent|SetSkeletalMesh (Variables|Default|GetM_ForeArm) _asskeletal_mesh_2 true)
                                (elif (Utilities|Enum|Equal(Enum) (.Slot (Utilities|Struct|BreakLuxSlotMeshData _array_element_3)) "EPS_Mandatory_UpperArm")
                                  (Class|SkinnedMeshComponent|SetSkeletalMesh (Variables|Default|GetM_UpperArm) _asskeletal_mesh_2 true)
                                  (elif (Utilities|Enum|Equal(Enum) (.Slot (Utilities|Struct|BreakLuxSlotMeshData _array_element_3)) "EPS_Mandatory_Shin")
                                    (Class|SkinnedMeshComponent|SetSkeletalMesh (Variables|Default|GetM_Shin) _asskeletal_mesh_2 true)
                                    (elif (Utilities|Enum|Equal(Enum) (.Slot (Utilities|Struct|BreakLuxSlotMeshData _array_element_3)) "EPS_Mandatory_Thigh")
                                      (Class|SkinnedMeshComponent|SetSkeletalMesh (Variables|Default|GetM_Thigh) _asskeletal_mesh_2 true)
                                      (elif (Utilities|Enum|Equal(Enum) (.Slot (Utilities|Struct|BreakLuxSlotMeshData _array_element_3)) "EPS_Mandatory_Knee")
                                        (Class|SkinnedMeshComponent|SetSkeletalMesh (Variables|Default|GetM_Knee) _asskeletal_mesh_2 true)
                                        (elif (Utilities|Enum|Equal(Enum) (.Slot (Utilities|Struct|BreakLuxSlotMeshData _array_element_3)) "EPS_Mandatory_Ankle")
                                          (Class|SkinnedMeshComponent|SetSkeletalMesh (Variables|Default|GetM_Ankle) _asskeletal_mesh_2 true)
                                          (elif (Utilities|Enum|Equal(Enum) (.Slot (Utilities|Struct|BreakLuxSlotMeshData _array_element_3)) "EPS_Optional_Head")
                                            (Class|SkinnedMeshComponent|SetSkeletalMesh (Variables|Default|GetO_Head) _asskeletal_mesh_2 true)
                                            (elif (Utilities|Enum|Equal(Enum) (.Slot (Utilities|Struct|BreakLuxSlotMeshData _array_element_3)) "EPS_Optional_Glasses")
                                              (Class|SkinnedMeshComponent|SetSkeletalMesh (Variables|Default|GetO_Glasses) _asskeletal_mesh_2 true)
                                              (elif (Utilities|Enum|Equal(Enum) (.Slot (Utilities|Struct|BreakLuxSlotMeshData _array_element_3)) "EPS_Optional_Necklace")
                                                (Class|SkinnedMeshComponent|SetSkeletalMesh (Variables|Default|GetO_Necklace) _asskeletal_mesh_2 true)
                                                (elif (Utilities|Enum|Equal(Enum) (.Slot (Utilities|Struct|BreakLuxSlotMeshData _array_element_3)) "EPS_Optional_ChestFit")
                                                  (Class|SkinnedMeshComponent|SetSkeletalMesh (Variables|Default|GetO_ChestFit) _asskeletal_mesh_2 true)
                                                  (elif (Utilities|Enum|Equal(Enum) (.Slot (Utilities|Struct|BreakLuxSlotMeshData _array_element_3)) "EPS_Optional_ChestPlate")
                                                    (Class|SkinnedMeshComponent|SetSkeletalMesh (Variables|Default|GetO_ChestPlate) _asskeletal_mesh_2 true)
                                                    (elif (Utilities|Enum|Equal(Enum) (.Slot (Utilities|Struct|BreakLuxSlotMeshData _array_element_3)) "EPS_Optional_BackCloth")
                                                      (Class|SkinnedMeshComponent|SetSkeletalMesh (Variables|Default|GetO_BackCloth) _asskeletal_mesh_2 true)
                                                      (elif (Utilities|Enum|Equal(Enum) (.Slot (Utilities|Struct|BreakLuxSlotMeshData _array_element_3)) "EPS_Optional_UpperArm")
                                                        (Class|SkinnedMeshComponent|SetSkeletalMesh (Variables|Default|GetO_UpperArm) _asskeletal_mesh_2 true)
                                                        (elif (Utilities|Enum|Equal(Enum) (.Slot (Utilities|Struct|BreakLuxSlotMeshData _array_element_3)) "EPS_Optional_Shoulder")
                                                          (Class|SkinnedMeshComponent|SetSkeletalMesh (Variables|Default|GetO_Shoulder) _asskeletal_mesh_2 true)
                                                          (elif (Utilities|Enum|Equal(Enum) (.Slot (Utilities|Struct|BreakLuxSlotMeshData _array_element_3)) "EPS_Optional_Gauntlet")
                                                            (Class|SkinnedMeshComponent|SetSkeletalMesh (Variables|Default|GetO_Gauntlet) _asskeletal_mesh_2 true)
                                                            (elif (Utilities|Enum|Equal(Enum) (.Slot (Utilities|Struct|BreakLuxSlotMeshData _array_element_3)) "EPS_Optional_UpperLeg")
                                                              (Class|SkinnedMeshComponent|SetSkeletalMesh (Variables|Default|GetO_UpperLeg) _asskeletal_mesh_2 true)
                                                              (elif (Utilities|Enum|Equal(Enum) (.Slot (Utilities|Struct|BreakLuxSlotMeshData _array_element_3)) "EPS_Optional_Skirt")
                                                                (Class|SkinnedMeshComponent|SetSkeletalMesh (Variables|Default|GetO_Skirt) _asskeletal_mesh_2 true)
                                                                (elif (Utilities|Enum|Equal(Enum) (.Slot (Utilities|Struct|BreakLuxSlotMeshData _array_element_3)) "EPS_Optional_Hem")
                                                                  (Class|SkinnedMeshComponent|SetSkeletalMesh (Variables|Default|GetO_Hem) _asskeletal_mesh_2 true)
                                                                  (elif (Utilities|Enum|Equal(Enum) (.Slot (Utilities|Struct|BreakLuxSlotMeshData _array_element_3)) "EPS_Optional_Belt")
                                                                    (Class|SkinnedMeshComponent|SetSkeletalMesh (Variables|Default|GetO_Belt) _asskeletal_mesh_2 true)
                                                                    (elif (Utilities|Enum|Equal(Enum) (.Slot (Utilities|Struct|BreakLuxSlotMeshData _array_element_3)) "EPS_Optional_Shoes")
                                                                      (Class|SkinnedMeshComponent|SetSkeletalMesh (Variables|Default|GetO_Shoes) _asskeletal_mesh_2 true)
                                                                      (elif (Utilities|Enum|Equal(Enum) (.Slot (Utilities|Struct|BreakLuxSlotMeshData _array_element_3)) "EPS_Optional_UnderShin")
                                                                        (Class|SkinnedMeshComponent|SetSkeletalMesh (Variables|Default|GetO_UnderShin) _asskeletal_mesh_2 true)
                                                                        (elif (Utilities|Enum|Equal(Enum) (.Slot (Utilities|Struct|BreakLuxSlotMeshData _array_element_3)) "EPS_Optional_Accessory")
                                                                          (Class|SkinnedMeshComponent|SetSkeletalMesh (Variables|Default|GetO_Accessory) _asskeletal_mesh_2 true)
                                                                          (elif (Utilities|Enum|Equal(Enum) (.Slot (Utilities|Struct|BreakLuxSlotMeshData _array_element_3)) "EPS_Optional_Cheek")
                                                                            (Class|SkinnedMeshComponent|SetSkeletalMesh (Variables|Default|GetO_Cheek) _asskeletal_mesh_2 true)
                                                                            (elif (Utilities|Enum|Equal(Enum) (.Slot (Utilities|Struct|BreakLuxSlotMeshData _array_element_3)) "EPS_Optional_Mantle")
                                                                              (Class|SkinnedMeshComponent|SetSkeletalMesh (Variables|Default|GetO_Mantle) _asskeletal_mesh_2 true)
                                                                              (elif (Utilities|Enum|Equal(Enum) (.Slot (Utilities|Struct|BreakLuxSlotMeshData _array_element_3)) "EPS_Optional_Maegami1")
                                                                                (Class|SkinnedMeshComponent|SetSkeletalMesh (Variables|Default|GetO_OptionalBangs1) _asskeletal_mesh_2 true)
                                                                                (elif (Utilities|Enum|Equal(Enum) (.Slot (Utilities|Struct|BreakLuxSlotMeshData _array_element_3)) "EPS_Optional_Maegami2")
                                                                                  (Class|SkinnedMeshComponent|SetSkeletalMesh (Variables|Default|GetO_OptionalBangs2) _asskeletal_mesh_2 true)
                                                                                  (elif (Utilities|Enum|Equal(Enum) (.Slot (Utilities|Struct|BreakLuxSlotMeshData _array_element_3)) "EPS_Racial_1")
                                                                                    (Class|SkinnedMeshComponent|SetSkeletalMesh (Variables|Default|GetRacial1) _asskeletal_mesh_2 true)
                                                                                    (elif (Utilities|Enum|Equal(Enum) (.Slot (Utilities|Struct|BreakLuxSlotMeshData _array_element_3)) "EPS_Racial_2")
                                                                                      (Class|SkinnedMeshComponent|SetSkeletalMesh (Variables|Default|GetRacial2) _asskeletal_mesh_2 true)
                                                                                      (elif (Utilities|Enum|Equal(Enum) (.Slot (Utilities|Struct|BreakLuxSlotMeshData _array_element_3)) "EPS_Racial_3")
                                                                                        (Class|SkinnedMeshComponent|SetSkeletalMesh (Variables|Default|GetRacial3) _asskeletal_mesh_2 true)
                                                                                        (elif (Utilities|Enum|Equal(Enum) (.Slot (Utilities|Struct|BreakLuxSlotMeshData _array_element_3)) "EPS_Racial_4")
                                                                                          (Class|SkinnedMeshComponent|SetSkeletalMesh (Variables|Default|GetRacial4) _asskeletal_mesh_2 true)))))))))))))))))))))))))))))))))))))))))))
      (elif (Utilities|Enum|Equal(Enum) (.Variation (Utilities|Struct|BreakLuxMeshDataVariation _array_element_2)) "EPV_B")
        (if (Utilities|Enum|Equal(Enum) _mesh_variation "EPV_B")
          (goto _label))
        (elif (Utilities|Enum|Equal(Enum) (.Variation (Utilities|Struct|BreakLuxMeshDataVariation _array_element_2)) "EPV_C")
          (if (Utilities|Enum|Equal(Enum) _mesh_variation "EPV_C")
            (goto _label))
          (elif (Utilities|Enum|Equal(Enum) (.Variation (Utilities|Struct|BreakLuxMeshDataVariation _array_element_2)) "EPV_D")
            (if (Utilities|Enum|Equal(Enum) _mesh_variation "EPV_D")
              (goto _label))
            (elif (Utilities|Enum|Equal(Enum) (.Variation (Utilities|Struct|BreakLuxMeshDataVariation _array_element_2)) "EPV_E")
              (if (Utilities|Enum|Equal(Enum) _mesh_variation "EPV_E")
                (goto _label))
              (elif (Utilities|Enum|Equal(Enum) (.Variation (Utilities|Struct|BreakLuxMeshDataVariation _array_element_2)) "EPV_F")
                (if (Utilities|Enum|Equal(Enum) _mesh_variation "EPV_F")
                  (goto _label))
                (elif (Utilities|Enum|Equal(Enum) (.Variation (Utilities|Struct|BreakLuxMeshDataVariation _array_element_2)) "EPV_G")
                  (if (Utilities|Enum|Equal(Enum) _mesh_variation "EPV_G")
                    (goto _label))
                  (elif (Utilities|Enum|Equal(Enum) (.Variation (Utilities|Struct|BreakLuxMeshDataVariation _array_element_2)) "EPV_H")
                    (if (Utilities|Enum|Equal(Enum) _mesh_variation "EPV_H")
                      (goto _label))
                    (elif (Utilities|Enum|Equal(Enum) (.Variation (Utilities|Struct|BreakLuxMeshDataVariation _array_element_2)) "EPV_Evil")
                      (if (Utilities|Enum|Equal(Enum) _mesh_variation "EPV_Evil")
                        (goto _label))
                      (elif (Utilities|Enum|Equal(Enum) (.Variation (Utilities|Struct|BreakLuxMeshDataVariation _array_element_2)) "EPV_Broken")
                        (if (Utilities|Enum|Equal(Enum) _mesh_variation "EPV_Broken")
                          (goto _label)))))))))))))
  (for _array_element_4 (Components|GetChildrenComponents (Variables|Default|GetDefaultSceneRoot) false)
    (bind _asskeletal_mesh_component (Utilities|Casting|CastToSkeletalMeshComponent _array_element_4))
    (for (_array_element_5 _array_index) (Rendering|Material|GetMaterials _asskeletal_mesh_component)
      (bind _returnvalue (Rendering|Material|CreateDynamicMaterialInstance _asskeletal_mesh_component _array_index _array_element_5 :!class /Script/Engine.PrimitiveComponent))
      (CallFunction|ColorDataFunc (Variables|ColorData|GetColorSlot1) _returnvalue "PatternColor 1" "PatternMask 1" "PatternNormal 1" "Pattern 1" _array_index _array_element_5)
      (CallFunction|ColorDataFunc (Variables|ColorData|GetColorSlot2) _returnvalue "PatternColor 2" "PatternMask 2" "PatternNormal 2" "Pattern 2" _array_index _array_element_5)
      (CallFunction|ColorDataFunc (Variables|ColorData|GetColorSlot3) _returnvalue "PatternColor 3" "PatternMask 3" "PatternNormal 3" "Pattern 3" _array_index _array_element_5)
      (CallFunction|ColorDataFunc (Variables|ColorData|GetColorSlot4) _returnvalue "PatternColor 4" "PatternMask 4" "PatternNormal 4" "Pattern 4" _array_index _array_element_5)
      (Rendering|Material|SetVectorParameterValueonMaterials _asskeletal_mesh_component "PatternValidMask" (Math|Conversions|ToVector(LinearColor) (Variables|ColorData|GetPatternValid%20Mask))))))

(fn ColorDataFunc
  (params (ColorData :type Color%20Data%20Structure) (DynamicMaterialInstance :type Material%20Instance%20Dynamic%20Object%20Reference) (PatternColor :type Name) (PatternMask :type Name) (PatternNormal :type Name) (Pattern%20# :type Name) (Element%20Index :type Integer) (MaterialInterface :type Material%20Interface%20Object%20Reference))
  (bind (_pattern _patterncolors _editableflags _size _rotate) (Utilities|Struct|BreakColorData ColorData))
  (bind _returnvalue (Utilities|String|ToString(Name) Pattern%20#))
  (bind _returnvalue_2 (Math|Float|Clamp(Float) _rotate -3.6e+02 3.6e+02))
  (bind _returnvalue_3 (Utilities|String|Append _returnvalue "" " Rotate"))
  (bind _returnvalue_4 (Utilities|String|Append _returnvalue "" " Color 1"))
  (bind _returnvalue_5 (Utilities|String|Append _returnvalue "" " Color 2"))
  (bind _returnvalue_6 (Utilities|String|Append _returnvalue "" " Color 3"))
  (bind _returnvalue_7 (Utilities|String|Append _returnvalue "" " Color 4"))
  (bind _returnvalue_8 (Utilities|String|Append _returnvalue "" " Size"))
  (bind _output (Utilities|Array|Get(acopy) _editableflags 3))
  (bind _output_2 (Utilities|Array|Get(acopy) _editableflags))
  (bind _output_3 (Utilities|Array|Get(acopy) _editableflags 1))
  (bind _output_4 (Utilities|Array|Get(acopy) _editableflags 2))
  (bind _output_5 (Utilities|Array|Get(acopy) _patterncolors 3))
  (bind _output_6 (Utilities|Array|Get(acopy) _patterncolors))
  (bind _output_7 (Utilities|Array|Get(acopy) _patterncolors 1))
  (bind _output_8 (Utilities|Array|Get(acopy) _patterncolors 2))
  (bind _sizemin (Variables|/Script/LuxorGame.LuxCreationTextureAsset|GetSizeMin _pattern))
  (bind _sizemax (Variables|/Script/LuxorGame.LuxCreationTextureAsset|GetSizeMax _pattern))
  (bind _normal (Variables|/Script/LuxorGame.LuxCreationTextureAsset|GetNormal _pattern))
  (bind _mask (Variables|/Script/LuxorGame.LuxCreationTextureAsset|GetMask _pattern))
  (bind _color (Variables|/Script/LuxorGame.LuxCreationTextureAsset|GetColor _pattern))
  (bind _returnvalue_9 (Math|Conversions|ToFloat(Boolean) _output_3))
  (bind _returnvalue_10 (Math|Conversions|ToFloat(Boolean) _output_2))
  (bind _returnvalue_11 (Math|Conversions|ToFloat(Boolean) _output_4))
  (bind _returnvalue_12 (Math|Conversions|ToFloat(Boolean) _output))
  (bind _returnvalue_13 (Utilities|String|StringToName _returnvalue_4))
  (bind _returnvalue_14 (Utilities|String|StringToName _returnvalue_5))
  (bind _returnvalue_15 (Utilities|String|StringToName _returnvalue_6))
  (bind _returnvalue_16 (Utilities|String|StringToName _returnvalue_3))
  (bind _returnvalue_17 (Utilities|String|StringToName _returnvalue_8))
  (bind _returnvalue_18 (Utilities|String|StringToName _returnvalue_7))
  (bind _returnvalue_19 (Math|Float|Clamp(Float) _size _sizemax _sizemin))
  (bind _linearcolor (Utilities|Struct|MakeLinearColor _returnvalue_10 _returnvalue_9 _returnvalue_11 _returnvalue_12))
  (bind _returnvalue_20 (Rendering|Material|GetScalarParameterValue DynamicMaterialInstance "IsSkin" :!class /Script/Engine.MaterialInstanceDynamic))
  (bind _returnvalue_21 (Rendering|Material|GetScalarParameterValue DynamicMaterialInstance "IsEyebrow" :!class /Script/Engine.MaterialInstanceDynamic))
  (bind _returnvalue_22 (Rendering|Material|GetScalarParameterValue DynamicMaterialInstance "IsBeard" :!class /Script/Engine.MaterialInstanceDynamic))
  (if (== _returnvalue_20 0.0)
    (if (== _returnvalue_21 0.0)
      (if (== _returnvalue_22 0.0)
        (Rendering|Material|SetTextureParameterValue DynamicMaterialInstance PatternColor _color)
        (Rendering|Material|SetTextureParameterValue DynamicMaterialInstance PatternMask _mask)
        (Rendering|Material|SetTextureParameterValue DynamicMaterialInstance PatternNormal _normal)
        (Rendering|Material|SetVectorParameterValue DynamicMaterialInstance (Utilities|String|StringToName (Utilities|String|Append _returnvalue "" " Flag")) _linearcolor :!class /Script/Engine.MaterialInstanceDynamic)
        (Rendering|Material|SetVectorParameterValue DynamicMaterialInstance _returnvalue_13 _output_6 :!class /Script/Engine.MaterialInstanceDynamic)
        (Rendering|Material|SetVectorParameterValue DynamicMaterialInstance _returnvalue_14 _output_7 :!class /Script/Engine.MaterialInstanceDynamic)
        (Rendering|Material|SetVectorParameterValue DynamicMaterialInstance _returnvalue_15 _output_8 :!class /Script/Engine.MaterialInstanceDynamic)
        (Rendering|Material|SetVectorParameterValue DynamicMaterialInstance _returnvalue_18 _output_5 :!class /Script/Engine.MaterialInstanceDynamic)
        (Rendering|Material|SetScalarParameterValue DynamicMaterialInstance _returnvalue_17 _returnvalue_19 :!class /Script/Engine.MaterialInstanceDynamic)
        (Rendering|Material|SetScalarParameterValue DynamicMaterialInstance _returnvalue_16 _returnvalue_2 :!class /Script/Engine.MaterialInstanceDynamic)))
    (else
      (bind _returnvalue_23 (Rendering|Material|CreateDynamicMaterialInstance (Variables|Default|GetM_Face) Element%20Index MaterialInterface :!class /Script/Engine.PrimitiveComponent))
      (Rendering|Material|SetTextureParameterValue _returnvalue_23 PatternColor _color)
      (Rendering|Material|SetTextureParameterValue _returnvalue_23 PatternMask _mask)
      (Rendering|Material|SetTextureParameterValue _returnvalue_23 PatternNormal _normal)
      (Rendering|Material|SetVectorParameterValue _returnvalue_23 _returnvalue_13 _linearcolor :!class /Script/Engine.MaterialInstanceDynamic)
      (Rendering|Material|SetVectorParameterValue _returnvalue_23 _returnvalue_13 _output_6 :!class /Script/Engine.MaterialInstanceDynamic)
      (Rendering|Material|SetVectorParameterValue _returnvalue_23 _returnvalue_14 _output_7 :!class /Script/Engine.MaterialInstanceDynamic)
      (Rendering|Material|SetVectorParameterValue _returnvalue_23 _returnvalue_15 _output_8 :!class /Script/Engine.MaterialInstanceDynamic)
      (Rendering|Material|SetVectorParameterValue _returnvalue_23 _returnvalue_18 _output_5 :!class /Script/Engine.MaterialInstanceDynamic)
      (Rendering|Material|SetScalarParameterValue _returnvalue_23 _returnvalue_17 _returnvalue_19 :!class /Script/Engine.MaterialInstanceDynamic)
      (Rendering|Material|SetScalarParameterValue _returnvalue_23 _returnvalue_16 _returnvalue_2 :!class /Script/Engine.MaterialInstanceDynamic))))